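; BP_SquareCButton is a square button actor in the collaborative buttons set that moves when another actor overlaps it.
; It caches its starting location on BeginPlay, then on overlap plays a timeline whose position output is added to that location.
; When an overlap ends, the timeline reverses from its end, so a partial press jumps to fully pressed before returning.
; The graph contains only this movement, with no overlap filtering.
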(event `self.ReceiveBeginPlay`
  (`parent.ReceiveBeginPlay`)
  (set `self.InitialLocation` (`self.K2_GetActorLocation`)))

(event `self.ReceiveActorBeginOverlap`
  (params (OtherActor :type "Actor Object Reference"))
  (bind (_direction _new_position) (`Timeline|OnPusheTimeline` :!label _label)
    (:`Update`
      (`self.K2_SetActorLocation` (+ _new_position (`self.InitialLocation`))))))

(event `self.ReceiveActorEndOverlap`
  (params (OtherActor :type "Actor Object Reference"))
  (goto _label :!via `ReverseFromEnd`))

(fn `UserConstructionScript`
  (`parent.UserConstructionScript`))