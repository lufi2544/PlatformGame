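; Base Blueprint for an overlap-triggered button that animates when pressed and applies or removes an effect.
; Overlap plays a timeline that offsets the actor from its start location unless IsButtonActive is set.
; Finishing forward calls ApplyEffect and flags the timer active; finishing in reverse calls UnApplyEffect.
; End overlap reverses at ReverseSpeed for unfinished presses or untimed position-only buttons; otherwise OnTimerFinish triggers release.
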(event `self.ReceiveBeginPlay`
  (set `self.InitialLocation` (`self.K2_GetActorLocation`)))

(event `self.ReceiveActorBeginOverlap`
  (params (OtherActor :type "Actor Object Reference"))
  (`self.ApplyTimeline`))

(event `self.ReceiveActorEndOverlap`
  (params (OtherActor :type "Actor Object Reference"))
  (`self.ApplyReverseTimeLine`))

(event `ApplyTimeline`
  (`TimelineComponent.SetPlayRate` (`self.EffectTimeline`) 6.0)
  (if (not (`self.bIsButtonActive`))
    (bind (_direction _new_location) (`Timeline|EffectTimeline` :!label _label)
      (:`Update`
        (`self.K2_SetActorLocation` (+ _new_location (`self.InitialLocation`))))
      (:`Finished`
        (if (`|EnumEquality` _direction "Forward")
          (`self.ApplyEffect`)
          (set `self.IsTimerActive` true)
          (else
            (`self.UnApplyEffect`)
            (`TimelineComponent.SetPlayRate` (`self.EffectTimeline`) 6.0)
            (set `self.IsTimerActive` false)))))))

(event `ApplyReverseTimeLine`
  (if (or (and (`self.bIsPositionOnly`) (not (`self.bHasTimer`))) (not (`self.IsTimerActive`)))
    (`TimelineComponent.SetPlayRate` (`self.EffectTimeline`) (`self.ReverseSpeed`) :!label _label_2)
    (goto _label :!via `Reverse`)))

(event `self.OnTimerFinish`
  (goto _label_2))

(fn `UserConstructionScript`)