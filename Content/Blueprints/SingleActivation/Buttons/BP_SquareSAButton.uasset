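; BP_SquareSAButton is a square single-activation button that moves when an actor overlaps it.
; A timeline offsets the button from the location stored at BeginPlay, playing forward on overlap.
; It reverses when overlap ends only if the button is position-only without a timer, or whenever the timer-finish event fires.
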(event `self.ReceiveBeginPlay`
  (set `self.InitialLocation` (`self.K2_GetActorLocation`)))

(event `self.ReceiveActorBeginOverlap`
  (params (OtherActor :type "Actor Object Reference"))
  (bind (_direction _new_location) (`Timeline|PushTimeline` :!label _label)
    (:`Update`
      (`self.K2_SetActorLocation` (+ _new_location (`self.InitialLocation`))))))

(event `self.ReceiveActorEndOverlap`
  (params (OtherActor :type "Actor Object Reference"))
  (if (and (`self.bIsPositionOnly`) (not (`self.bHasTimer`)))
    (goto _label :!via `Reverse`)))

(event `self.OnTimerFinish`
  (goto _label :!via `Reverse`))

(fn `UserConstructionScript`
  (`parent.UserConstructionScript`))